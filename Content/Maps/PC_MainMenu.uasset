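; PC_MainMenu is the main menu player controller, which can create and remove a HUD widget.
; SetupGameHUD creates W_InGameHUD for a local player controller, stores it and adds it to the viewport, and EndPlay removes it from its parent.
; ClientPostLoginEvent only casts the game mode to GM_MainMenu, and nothing in this graph calls SetupGameHUD.
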(event Custom|ClientPostLoginEvent
  ;[1 1 1] Adds hud to only 1 client
  (Utilities|Casting|CastToGM_MainMenu (Game|GetGameMode)))

(event EventBeginPlay)

(event EventTick
  (params (DeltaSeconds :type Float%20%28single-precision%29)))

(event EventEndPlay
  (params (EndPlayReason :type EEndPlayReason%20Enum :default "Destroyed"))
  ;[1 1 1] Removes hud when leaving level
  (Widget|RemovefromParent (Variables|Default|GetHud)))

(fn ConstructionScript)

(fn SetupGameHUD
  (if (Pawn|IsLocalPlayerController)
    (bind _returnvalue (UserInterface|CreateWidget "/Game/PlayerCharacter/Blueprints/Multiplayer/Widgets/W_InGameHUD.W_InGameHUD_C" self))
    (bind _output_get (Variables|Default|SetHud _returnvalue))
    (UserInterface|Viewport|AddtoViewport _output_get 0)))