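; VR player character for placing road tiles on a grid and switching between two world scales.
; Right face buttons spawn static mesh components from the right controller's ground-plane position, tracking state with Selected and RoadSelected.
; AttachToHand and the left trigger snap those meshes to a 100-unit grid.
; Either grip toggles zoom by changing world-to-meters scale, resizing controller meshes and moving the actor to the head position or world origin.
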(event Custom|ReceiveTick_Copy
  (params (DeltaSeconds :type Float%20%28single-precision%29 :default 0.0))
  (CallFunction|AttachtoHand (stale Input|KeyboardEvents|MotionControllerRightFaceButton1 _returnvalue) (stale Input|KeyboardEvents|MotionControllerRightFaceButton1 _x) (stale Input|KeyboardEvents|MotionControllerRightFaceButton1 _y) (Variables|Default|GetRoadSelected)))

(event Input|KeyboardEvents|MotionControllerRightTrigger
  (params (Key :type Key%20Structure :default "AnyKey"))
  ;[1 1 1] Pickup Object w/ Triggers
  ; (Trigger Events could be Inputs instead if you wanted)
)

(event Input|KeyboardEvents|MotionControllerLeftTrigger
  (params (Key :type Key%20Structure :default "AnyKey"))
  ;[1 1 1] Pickup Object w/ Triggers
  ; (Trigger Events could be Inputs instead if you wanted)
  (:Pressed
    (Development|PrintString "Pressed")))

(event Input|KeyboardEvents|MotionControllerRightFaceButton3
  (params (Key :type Key%20Structure :default "AnyKey"))
  (:Pressed
    (Variables|Default|SetTest "0.000000, 0, 0")))

(event Input|KeyboardEvents|MotionControllerRightFaceButton1
  (params (Key :type Key%20Structure :default "AnyKey"))
  (:Pressed
    (bind (_x _y) (CallFunction|SpawnTile (Variables|Default|GetSelected) (Variables|Default|GetRoadSelected)))
    (bind _returnvalue (AddComponent|AddStaticMeshComponent false (Math|Conversions|ToTransform(Vector) (Math|Vector|MakeVector _x _y 0.0))))
    (Variables|Default|SetSelected false)
    (Variables|Default|SetRoadSelected true)))

(event Input|KeyboardEvents|MotionControllerRightFaceButton2
  (params (Key :type Key%20Structure :default "AnyKey"))
  (bind _r_motioncontroller (Variables|Default|GetR_MotionController))
  (bind _returnvalue (Transformation|GetWorldLocation _r_motioncontroller))
  (bind _returnvalue_2 (* _returnvalue "1.000000,1.000000,0.0"))
  (:Pressed
    (if (not (Variables|Default|GetSelected))
      (bind _returnvalue_3 (AddComponent|AddStaticMeshComponent false (Math|Conversions|ToTransform(Vector) (Math|Vector|MakeVector (.x _returnvalue_2) (.y _returnvalue_2) (.z _returnvalue_2))))))))

(event Input|KeyboardEvents|MotionControllerLeftTrigger
  (params (Key :type Key%20Structure :default "AnyKey"))
  (bind _100 (Variables|Default|Get100))
  (bind _r_motioncontroller (Variables|Default|GetR_MotionController))
  (bind _returnvalue (Transformation|GetWorldLocation _r_motioncontroller))
  (bind _returnvalue_2 (* _returnvalue "1.000000,1.000000,0.0"))
  (:Pressed
    (Variables|Default|SetSelected false)
    (if (Variables|Default|GetRoadSelected)
      (Transformation|SetWorldLocation (stale Input|KeyboardEvents|MotionControllerRightFaceButton2 _returnvalue_3) (Math|Vector|MakeVector (* (Math|Float|Round (/ (.x _returnvalue_2) _100)) _100) (* (Math|Float|Round (/ (.y _returnvalue_2) _100)) _100) 0.0) false false))))

(event Input|KeyboardEvents|MotionControllerRightGrip1
  (params (Key :type Key%20Structure :default "AnyKey"))
  (bind _0 (Variables|Default|Get0))
  (bind _10 (Variables|Default|Get10))
  (bind __1 (Variables|Default|Get.1))
  (:Pressed
    (if (Variables|Default|GetZoomed)
      (Class|HeadMountedDisplayFunctionLibrary|SetWorldtoMetersScale 1e+03)
      (Variables|Default|SetZoomed false)
      (Transformation|SetWorldScale3D (Variables|Default|GetL_ViveMesh) (Math|Vector|MakeVector _10 _10 _10))
      (Transformation|SetActorLocation (Transformation|GetWorldLocation (Variables|Default|GetHead)) true false)
      (else
        (Class|HeadMountedDisplayFunctionLibrary|SetWorldtoMetersScale 1e+02)
        (Variables|Default|SetZoomed true)
        (Transformation|SetWorldScale3D (Variables|Default|GetL_ViveMesh) (Math|Vector|MakeVector __1 __1 __1))
        (Transformation|SetActorLocation (Math|Vector|MakeVector _0 _0 _0) true false)))))

(event Input|KeyboardEvents|MotionControllerLeftGrip1
  (params (Key :type Key%20Structure :default "AnyKey"))
  (bind _0 (Variables|Default|Get0))
  (bind _10 (Variables|Default|Get10))
  (bind __1 (Variables|Default|Get.1))
  (:Pressed
    (if (Variables|Default|GetZoomed)
      (Class|HeadMountedDisplayFunctionLibrary|SetWorldtoMetersScale 1e+03)
      (Variables|Default|SetZoomed false)
      (Transformation|SetWorldScale3D (Variables|Default|GetL_ViveMesh) (Math|Vector|MakeVector _10 _10 _10))
      (Transformation|SetActorLocation (Transformation|GetWorldLocation (Variables|Default|GetHead)) true false)
      (else
        (Class|HeadMountedDisplayFunctionLibrary|SetWorldtoMetersScale 1e+02)
        (Variables|Default|SetZoomed true)
        (Transformation|SetWorldScale3D (Variables|Default|GetL_ViveMesh) (Math|Vector|MakeVector __1 __1 __1))
        (Transformation|SetActorLocation (Math|Vector|MakeVector _0 _0 _0) true false)))))

(fn ConstructionScript)

(fn SpawnTile
  (params (Any%20Selected :type Boolean) (Selected%20Tile :type Boolean))
  (bind _r_motioncontroller (Variables|Default|GetR_MotionController))
  (bind _returnvalue (Transformation|GetWorldLocation _r_motioncontroller))
  (if (not Any%20Selected)
    (return (.x _returnvalue) (.y _returnvalue))))

(fn AttachtoHand
  (params (SceneComponent :type Scene%20Component%20Object%20Reference) (x :type Float%20%28single-precision%29) (y :type Float%20%28single-precision%29) (Selected%20Tile :type Boolean))
  (bind _100 (Variables|Default|Get100))
  (if Selected%20Tile
    (Transformation|SetWorldLocation SceneComponent (Math|Vector|MakeVector (* (Math|Float|Round (/ x _100)) _100) (* (Math|Float|Round (/ y _100)) _100) 0.0) false false)))