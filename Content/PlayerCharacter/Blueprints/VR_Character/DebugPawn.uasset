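; Debug pawn for grid-based city building, placing Road and Commercial tiles with keys and mouse.
; Tick snaps the selected tile to a 100-unit grid via a view line trace.
; Left-click validates placement, turning overlaps red or setting the tile's material and storing it; right-click destroys the selection.
; Roads record neighbour links as compass-letter strings, which choose straight, corner or intersection materials, rotating only east-west straights.
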(event EventBeginPlay)

(event EventActorBeginOverlap
  (params (OtherActor :type Actor%20Object%20Reference)))

(event EventTick
  (params (DeltaSeconds :type Float%20%28single-precision%29))
  (bind _floor_location (CallFunction|FloorLocation))
  (Variables|Default|SetFloorTransform (Math|Conversions|ToTransform(Vector) _floor_location))
  (if (!= (Variables|Default|GetSelected%20Tile) 0)
    (Transformation|SetActorLocation (Variables|Default|GetSelected%20Tile) _floor_location false false)))

(event Input|KeyboardEvents|1
  (params (Key :type Key%20Structure :default "AnyKey"))
  (:Pressed
    (Actor|DestroyActor (Variables|Default|GetSelected%20Tile))
    (bind _returnvalue (Game|SpawnActorfromClass "/Game/LevelContent/Meshes/Road/Road.Road_C" (Variables|Default|GetFloorTransform) "Undefined" 0 0))
    (Variables|Default|SetSelected%20Tile _returnvalue)))

(event Input|KeyboardEvents|2
  (params (Key :type Key%20Structure :default "AnyKey"))
  (:Pressed
    (Actor|DestroyActor (Variables|Default|GetSelected%20Tile))
    (bind _returnvalue (Game|SpawnActorfromClass "/Game/LevelContent/Meshes/Commercial/Commercial.Commercial_C" (Variables|Default|GetFloorTransform) "Undefined" 0 0))
    (Variables|Default|SetSelected%20Tile _returnvalue)))

(event Input|MouseEvents|RightMouseButton
  (params (Key :type Key%20Structure :default "AnyKey"))
  (:Pressed
    (if (!= (Variables|Default|GetSelected%20Tile) 0)
      (Actor|DestroyActor (Variables|Default|GetSelected%20Tile)))))

(event Input|MouseEvents|LeftMouseButton
  (params (Key :type Key%20Structure :default "AnyKey"))
  (:Pressed
    (if (!= (Variables|Default|GetSelected%20Tile) 0)
      (bind _allowed (CallFunction|ValidateTile (Variables|Default|GetTiles) (Variables|Default|GetSelected%20Tile)))
      (if _allowed
        (Utilities|Array|Add (Variables|Default|GetTiles) (Variables|Default|GetSelected%20Tile))
        (Variables|Default|SetSelected%20Tile 0)))))

(fn ConstructionScript)

(fn FloorLocation
  (bind (_outlocation _outrotation) (Actor|GetActorEyesViewPoint))
  (bind _100 (Variables|Default|Get100))
  (bind _outhit (Collision|LineTraceByChannel _outlocation (+ _outlocation (* (Math|Vector|GetForwardVector _outrotation) 50000)) "TraceTypeQuery1" false 0 "None"))
  (return (Math|Vector|MakeVector (* (Math|Float|Round (/ (.x (* (.ImpactPoint (Collision|BreakHitResult _outhit)) "1.000000,1.000000,0.0")) _100)) _100) (* (Math|Float|Round (/ (.y (* (.ImpactPoint (Collision|BreakHitResult _outhit)) "1.000000,1.000000,0.0")) _100)) _100) 0.0)))

(fn ValidateTile
  (params (Tile%20Array :type Array%20of%20Actor%20Object%20References) (New%20Tile :type Actor%20Object%20Reference))
  (bind _returnvalue (VehicleSound|GetRootComponent New%20Tile))
  (LocalVariables|SetIsAllowed true)
  (for _array_element Tile%20Array
    (if (Math|Vector|Equal(Vector) (Transformation|GetWorldLocation _returnvalue) (Transformation|GetWorldLocation (VehicleSound|GetRootComponent _array_element)) 0.0001)
      (bind _asprimitive_component (Utilities|Casting|CastToPrimitiveComponent (Components|GetChildComponent _returnvalue 0))
        (:then
          (Rendering|Material|SetMaterial _asprimitive_component 0 "/Game/PlayerCharacter/Blueprints/VR_Character/REd.REd"))
        (:CastFailed
          _))
      (LocalVariables|SetIsAllowed false)
      (return (LocalVariables|GetIsAllowed))))
  (CallFunction|SetMaterial New%20Tile)
  (return (LocalVariables|GetIsAllowed)))

(fn SetMaterial
  (params (New%20Tile :type Actor%20Object%20Reference))
  (if (Actor|ActorHasTag New%20Tile "Commercial")
    (bind _asprimitive_component (Utilities|Casting|CastToPrimitiveComponent (Components|GetChildComponent (VehicleSound|GetRootComponent New%20Tile) 0))
      (:then
        _)
      (:CastFailed
        _))
    (Rendering|Material|SetMaterial _asprimitive_component 0 "/Game/LevelContent/Material.Material")
    (elif (Actor|ActorHasTag New%20Tile "Road")
      (CallFunction|RoadManager New%20Tile)
      (else
        (Development|PrintString "Tags not working"))))
  (return))

(fn RoadManager
  (params (New%20Tile :type Actor%20Object%20Reference))
  (bind _road_branches (Variables|Default|GetRoad%20Branches))
  (for (_array_element _array_index) (Variables|Default|GetRoads)
    (if (Math|Float|NearlyEqual(Float) (Transformation|GetDistanceTo New%20Tile _array_element) 1e+02 0.1)
      (if (Math|Float|NearlyEqual(Float) (.x (- (Transformation|GetWorldLocation (Components|GetChildComponent (VehicleSound|GetRootComponent _array_element) 0)) (Transformation|GetWorldLocation (Components|GetChildComponent (VehicleSound|GetRootComponent New%20Tile) 0)))) 1e+02 0.1)
        (Utilities|Array|SetArrayElem _road_branches _array_index (Utilities|String|Append (Utilities|Array|Get(acopy) _road_branches _array_index) "N") true)
        (LocalVariables|SetNew%20Road (Utilities|String|Append (LocalVariables|GetNew%20Road) "S"))
        (CallFunction|AddRoad _array_index)
        (elif (Math|Float|NearlyEqual(Float) (.x (- (Transformation|GetWorldLocation (Components|GetChildComponent (VehicleSound|GetRootComponent _array_element) 0)) (Transformation|GetWorldLocation (Components|GetChildComponent (VehicleSound|GetRootComponent New%20Tile) 0)))) -1e+02 0.1)
          (Utilities|Array|SetArrayElem _road_branches _array_index (Utilities|String|Append (Utilities|Array|Get(acopy) _road_branches _array_index) "S") true)
          (LocalVariables|SetNew%20Road (Utilities|String|Append (LocalVariables|GetNew%20Road) "N"))
          (CallFunction|AddRoad _array_index)
          (elif (Math|Float|NearlyEqual(Float) (.y (- (Transformation|GetWorldLocation (Components|GetChildComponent (VehicleSound|GetRootComponent _array_element) 0)) (Transformation|GetWorldLocation (Components|GetChildComponent (VehicleSound|GetRootComponent New%20Tile) 0)))) 1e+02 0.1)
            (Utilities|Array|SetArrayElem _road_branches _array_index (Utilities|String|Append (Utilities|Array|Get(acopy) _road_branches _array_index) "E") true)
            (LocalVariables|SetNew%20Road (Utilities|String|Append (LocalVariables|GetNew%20Road) "W"))
            (CallFunction|AddRoad _array_index)
            (elif (Math|Float|NearlyEqual(Float) (.y (- (Transformation|GetWorldLocation (Components|GetChildComponent (VehicleSound|GetRootComponent _array_element) 0)) (Transformation|GetWorldLocation (Components|GetChildComponent (VehicleSound|GetRootComponent New%20Tile) 0)))) -1e+02 0.1)
              (Utilities|Array|SetArrayElem _road_branches _array_index (Utilities|String|Append (Utilities|Array|Get(acopy) _road_branches _array_index) "W") true)
              (LocalVariables|SetNew%20Road (Utilities|String|Append (LocalVariables|GetNew%20Road) "E"))
              (CallFunction|AddRoad _array_index)))))))
  (Utilities|Array|Add (Variables|Default|GetRoads) New%20Tile)
  (Utilities|Array|Add (Variables|Default|GetRoad%20Branches) (LocalVariables|GetNew%20Road))
  (CallFunction|AddRoad (Utilities|Array|LastIndex (Variables|Default|GetRoads)))
  (return))

(fn AddRoad
  (params (Index :type Integer))
  (bind _roads (Variables|Default|GetRoads))
  (bind _item (Utilities|Array|Get(acopy) _roads Index))
  (LocalVariables|SetTile _item)
  (bind _output_get (LocalVariables|SetArrayChar (Utilities|String|GetCharacterArrayfromString (Utilities|Array|Get(acopy) (Variables|Default|GetRoad%20Branches) Index))))
  (bind _asprimitive_component (Utilities|Casting|CastToPrimitiveComponent (Components|GetChildComponent (VehicleSound|GetRootComponent _item) 0))
    (:then
      (if (== (Utilities|Array|Length _output_get) 4)
        (Rendering|Material|SetMaterial _asprimitive_component 0 "/Game/LevelContent/Meshes/Road/Mat_Intersection4.Mat_Intersection4")
        (elif (== (Utilities|Array|Length _output_get) 3)
          (Rendering|Material|SetMaterial _asprimitive_component 0 "/Game/LevelContent/Meshes/Road/Mat_Intersection3.Mat_Intersection3")
          (elif (== (Utilities|Array|Length _output_get) 2)
            (if (or (and (Utilities|Array|ContainsItem (LocalVariables|GetArrayChar) (Utilities|String|ToString(Name) "W")) (Utilities|Array|ContainsItem (LocalVariables|GetArrayChar) (Utilities|String|ToString(Name) "E"))) (and (Utilities|Array|ContainsItem (LocalVariables|GetArrayChar) (Utilities|String|ToString(Name) "N")) (Utilities|Array|ContainsItem (LocalVariables|GetArrayChar) (Utilities|String|ToString(Name) "S"))))
              (Rendering|Material|SetMaterial _asprimitive_component 0 "/Game/LevelContent/Meshes/Road/Mat_Road1.Mat_Road1" :!label _label)
              (if (and (Utilities|Array|ContainsItem (LocalVariables|GetArrayChar) (Utilities|String|ToString(Name) "W")) (Utilities|Array|ContainsItem (LocalVariables|GetArrayChar) (Utilities|String|ToString(Name) "E")))
                (Transformation|SetActorRotation (LocalVariables|GetTile) "0,90.000000, 0"))
              (else
                (Rendering|Material|SetMaterial _asprimitive_component 0 "/Game/LevelContent/Meshes/Road/Mat_Corner2.Mat_Corner2")))
            (elif (== (Utilities|Array|Length _output_get) 1)
              (goto _label)
              (else
                (Development|PrintString "Invalid Road Connections")))))))
    (:CastFailed
      (Development|PrintString "Cast Failed")))
  (return))